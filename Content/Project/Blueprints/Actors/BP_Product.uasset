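; BP_Product is an interactable product actor that shows its info on the HUD when looked at.
; The construction script applies its configured mesh, and BeginPlay caches the BP_HUD from the player controller.
; LookAt enables custom depth rendering on the mesh and sends the product info to the HUD, while LookAway clears both.
; Interact clears the HUD text, destroys the actor and returns its product info to the caller.
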(event EventLookAway
  (Rendering|SetRenderCustomDepth (Variables|Default|GetStaticMesh) false)
  (Default|SetProductOutTexts (Variables|Default|GetHUD%20Reference)))

(event EventBeginPlay
  (bind _asbp_hud (Utilities|Casting|CastToBP_HUD (HUD|GetHUD (Game|GetPlayerController 0))))
  (Variables|Default|SetHUD%20Reference _asbp_hud))

(fn ConstructionScript
  (Components|StaticMesh|SetStaticMesh (Variables|Default|GetStaticMesh) (Variables|Default|GetMesh)))

(fn Interact
  (Default|SetProductOutTexts (Variables|Default|GetHUD%20Reference))
  (Actor|DestroyActor)
  (return (Variables|Default|GetProductInfo)))

(fn Lookat
  (Rendering|SetRenderCustomDepth (Variables|Default|GetStaticMesh) true)
  (Default|SetProductOutTexts (Variables|Default|GetHUD%20Reference) (Variables|Default|GetProductInfo))
  (return (Variables|Default|GetProductInfo)))