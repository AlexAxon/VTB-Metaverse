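; Parent sliding double-door actor that opens and closes two panels along their relative X axis.
; OpenDoor disables box collision and plays a timeline whose eased alpha offsets both panels oppositely from cached start positions, up to MaxOpenWidth.
; CloseDoor restores collision and reverses that timeline, and CloseDoorAfterEnter calls it when given a BP_Character.
; BeginPlay also caches the HUD and sets initial collision, with EnableCollisiomOnStart inverted: true means no collision.
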(event Custom|OpenDoor
  (bind _leftdoorstartlocation (Variables|Default|GetLeftDoorStartLocation))
  (bind _rightdoorstartlocation (Variables|Default|GetRightDoorStartLocation))
  ;[1 0 0] Открытие и закрытие двери
  (Variables|Default|SetbIsOpen true)
  (Collision|SetCollisionEnabled (Variables|Default|GetBoxCollision) "NoCollision")
  (bind _alpha (Timeline|Timeline_Open_Door Play)
    (:Update
      (Variables|Default|SetCurrentOpenWidth (Math|Interpolation|Ease (Variables|Default|GetFunctionInterpolation) _alpha 0.0 (Variables|Default|GetMaxOpenWidth) 2.0))
      (Transformation|SetRelativeLocation (Variables|Default|GetRightDoor) (Math|Vector|MakeVector (+ (.x _rightdoorstartlocation) (Variables|Default|GetCurrentOpenWidth)) (.y _rightdoorstartlocation) (.z _rightdoorstartlocation)) false false)
      (Transformation|SetRelativeLocation (Variables|Default|GetLeftDoor) (Math|Vector|MakeVector (- (.x _leftdoorstartlocation) (Variables|Default|GetCurrentOpenWidth)) (.y _leftdoorstartlocation) (.z _leftdoorstartlocation)) false false))))

(event Custom|CloseDoor
  (bind _leftdoorstartlocation (Variables|Default|GetLeftDoorStartLocation))
  (bind _rightdoorstartlocation (Variables|Default|GetRightDoorStartLocation))
  ;[1 0 0] Открытие и закрытие двери
  (Variables|Default|SetbIsOpen false)
  (Collision|SetCollisionEnabled (Variables|Default|GetBoxCollision) "QueryAndPhysics")
  (bind _alpha (Timeline|Timeline_Open_Door Reverse)
    (:Update
      (Variables|Default|SetCurrentOpenWidth (Math|Interpolation|Ease (Variables|Default|GetFunctionInterpolation) _alpha 0.0 (Variables|Default|GetMaxOpenWidth) 2.0))
      (Transformation|SetRelativeLocation (Variables|Default|GetRightDoor) (Math|Vector|MakeVector (+ (.x _rightdoorstartlocation) (Variables|Default|GetCurrentOpenWidth)) (.y _rightdoorstartlocation) (.z _rightdoorstartlocation)) false false)
      (Transformation|SetRelativeLocation (Variables|Default|GetLeftDoor) (Math|Vector|MakeVector (- (.x _leftdoorstartlocation) (Variables|Default|GetCurrentOpenWidth)) (.y _leftdoorstartlocation) (.z _leftdoorstartlocation)) false false))))

(event EventBeginPlay
  (Variables|Default|SetLeftDoorStartLocation (Variables|/Script/Engine.SceneComponent|GetRelativeLocation (Variables|Default|GetLeftDoor)))
  (Variables|Default|SetRightDoorStartLocation (Variables|/Script/Engine.SceneComponent|GetRelativeLocation (Variables|Default|GetRightDoor)))
  (Collision|SetCollisionEnabled (Variables|Default|GetBoxCollision) (select (Variables|Default|GetbEnableCollisiomOnStart) "NoCollision" "QueryAndPhysics"))
  (bind _asbp_hud (Utilities|Casting|CastToBP_HUD (HUD|GetHUD (Game|GetPlayerController 0))))
  (Variables|Default|SetHUD%20Reference _asbp_hud))

(fn ConstructionScript)

(fn CloseDoorAfterEnter
  (params (ActorReference :type Actor%20Object%20Reference))
  (Utilities|Casting|CastToBP_Character ActorReference)
  (CallFunction|CloseDoor))