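; BP_EnterDoor is a sliding double-door actor that opens as BP_Character enters and closes behind it.
; Overlapping EnterBoxCollision plays a timeline that slides both doors apart along relative X from positions cached at BeginPlay.
; Overlapping ExitBoxCollision reverses that timeline and enables BoxCollision, which starts disabled and is never switched off again afterwards.
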(event OnComponentBeginOverlap(EnterBoxCollision)
  (params (OverlappedComponent :type Primitive%20Component%20Object%20Reference) (OtherActor :type Actor%20Object%20Reference) (OtherComp :type Primitive%20Component%20Object%20Reference) (OtherBodyIndex :type Integer) (bFromSweep :type Boolean) (SweepResult :type Hit%20Result%20Structure%20%28by%20ref%29))
  (Utilities|Casting|CastToBP_Character OtherActor)
  (CallFunction|OpenDoor))

(event OnComponentBeginOverlap(ExitBoxCollision)
  (params (OverlappedComponent :type Primitive%20Component%20Object%20Reference) (OtherActor :type Actor%20Object%20Reference) (OtherComp :type Primitive%20Component%20Object%20Reference) (OtherBodyIndex :type Integer) (bFromSweep :type Boolean) (SweepResult :type Hit%20Result%20Structure%20%28by%20ref%29))
  (Utilities|Casting|CastToBP_Character OtherActor)
  (CallFunction|CloseDoor)
  (Collision|SetCollisionEnabled (Variables|Default|GetBoxCollision) "QueryAndPhysics"))

(event Custom|OpenDoor
  (bind _leftdoorstartlocation (Variables|Default|GetLeftDoorStartLocation))
  (bind _rightdoorstartlocation (Variables|Default|GetRightDoorStartLocation))
  (bind _open_width (Timeline|Timeline_Open_Door Play)
    (:Update
      (Transformation|SetRelativeLocation (Variables|Default|GetRightDoor) (Math|Vector|MakeVector (+ (.x _rightdoorstartlocation) _open_width) (.y _rightdoorstartlocation) (.z _rightdoorstartlocation)) false false)
      (Transformation|SetRelativeLocation (Variables|Default|GetLeftDoor) (Math|Vector|MakeVector (- (.x _leftdoorstartlocation) _open_width) (.y _leftdoorstartlocation) (.z _leftdoorstartlocation)) false false))))

(event Custom|CloseDoor
  (bind _leftdoorstartlocation (Variables|Default|GetLeftDoorStartLocation))
  (bind _rightdoorstartlocation (Variables|Default|GetRightDoorStartLocation))
  (bind _open_width (Timeline|Timeline_Open_Door Reverse)
    (:Update
      (Transformation|SetRelativeLocation (Variables|Default|GetRightDoor) (Math|Vector|MakeVector (+ (.x _rightdoorstartlocation) _open_width) (.y _rightdoorstartlocation) (.z _rightdoorstartlocation)) false false)
      (Transformation|SetRelativeLocation (Variables|Default|GetLeftDoor) (Math|Vector|MakeVector (- (.x _leftdoorstartlocation) _open_width) (.y _leftdoorstartlocation) (.z _leftdoorstartlocation)) false false))))

(event EventBeginPlay
  (Variables|Default|SetLeftDoorStartLocation (Variables|/Script/Engine.SceneComponent|GetRelativeLocation (Variables|Default|GetLeftDoor)))
  (Variables|Default|SetRightDoorStartLocation (Variables|/Script/Engine.SceneComponent|GetRelativeLocation (Variables|Default|GetRightDoor)))
  (Collision|SetCollisionEnabled (Variables|Default|GetBoxCollision) "NoCollision"))

(event EventTick
  (params (DeltaSeconds :type Float%20%28single-precision%29)))

(fn ConstructionScript)