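; BP_SecondDoor is the exit door that opens once the player has taken enough products.
; It binds to the character's GetProduct event on BeginPlay, then opens once and shows a goal-completed notification when the product count reaches the minimum.
; Three exit collision boxes call CloseDoorAfterEnter and share a one-shot that fires the close-door call, shows a farewell notification and hides the HUD product list.
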(event OnComponentBeginOverlap(ExitBoxCollision)
  (params (OverlappedComponent :type Primitive%20Component%20Object%20Reference) (OtherActor :type Actor%20Object%20Reference) (OtherComp :type Primitive%20Component%20Object%20Reference) (OtherBodyIndex :type Integer) (bFromSweep :type Boolean) (SweepResult :type Hit%20Result%20Structure%20%28by%20ref%29))
  (CallFunction|CloseDoorAfterEnter OtherActor)
  (Utilities|FlowControl|DoOnce false
    (:Completed
      (Default|CallOnCloseDoor)
      (Default|PlayNotification (Variables|Default|GetHUD%20Reference) "Спасибо за посещение")
      (Widget|SetVisibility (Variables|/Game/Project/Blueprints/UMG/UMG_MainUI.UMG_MainUI_C|GetBorder_ProductList (Variables|/Game/Project/Blueprints/Core/BP_HUD.BP_HUD_C|GetMainUI%20Reference (Variables|/Game/Project/Blueprints/Core/BP_Character.BP_Character_C|GetHUD%20Reference (Variables|Default|GetAs%20BP%20Character)))) "Hidden"))))

(event OnComponentBeginOverlap(ExitBoxCollision1)
  (params (OverlappedComponent :type Primitive%20Component%20Object%20Reference) (OtherActor :type Actor%20Object%20Reference) (OtherComp :type Primitive%20Component%20Object%20Reference) (OtherBodyIndex :type Integer) (bFromSweep :type Boolean) (SweepResult :type Hit%20Result%20Structure%20%28by%20ref%29))
  (CallFunction|CloseDoorAfterEnter OtherActor)
  (Utilities|FlowControl|DoOnce false
    (:Completed
      (Default|CallOnCloseDoor)
      (Default|PlayNotification (Variables|Default|GetHUD%20Reference) "Спасибо за посещение")
      (Widget|SetVisibility (Variables|/Game/Project/Blueprints/UMG/UMG_MainUI.UMG_MainUI_C|GetBorder_ProductList (Variables|/Game/Project/Blueprints/Core/BP_HUD.BP_HUD_C|GetMainUI%20Reference (Variables|/Game/Project/Blueprints/Core/BP_Character.BP_Character_C|GetHUD%20Reference (Variables|Default|GetAs%20BP%20Character)))) "Hidden"))))

(event OnComponentBeginOverlap(ExitBoxCollision2)
  (params (OverlappedComponent :type Primitive%20Component%20Object%20Reference) (OtherActor :type Actor%20Object%20Reference) (OtherComp :type Primitive%20Component%20Object%20Reference) (OtherBodyIndex :type Integer) (bFromSweep :type Boolean) (SweepResult :type Hit%20Result%20Structure%20%28by%20ref%29))
  (CallFunction|CloseDoorAfterEnter OtherActor)
  (Utilities|FlowControl|DoOnce false
    (:Completed
      (Default|CallOnCloseDoor)
      (Default|PlayNotification (Variables|Default|GetHUD%20Reference) "Спасибо за посещение")
      (Widget|SetVisibility (Variables|/Game/Project/Blueprints/UMG/UMG_MainUI.UMG_MainUI_C|GetBorder_ProductList (Variables|/Game/Project/Blueprints/Core/BP_HUD.BP_HUD_C|GetMainUI%20Reference (Variables|/Game/Project/Blueprints/Core/BP_Character.BP_Character_C|GetHUD%20Reference (Variables|Default|GetAs%20BP%20Character)))) "Hidden"))))

(event Custom|CountingProductsTaken
  (if (>= (Variables|/Game/Project/Blueprints/Core/BP_Character.BP_Character_C|GetProductsCount (Variables|Default|GetAs%20BP%20Character)) (Variables|Default|GetMinNumberOfProducts))
    (Utilities|FlowControl|DoOnce false
      (:Completed
        (CallFunction|OpenDoor)
        (Default|PlayNotification (Variables|Default|GetHUD%20Reference) "Цель выполнена и выход открылся")))))

(event EventBeginPlay
  (|CallParentFunction)
  (bind _asbp_character (Utilities|Casting|CastToBP_Character (Game|Player|GetPlayerPawn 0)))
  (bind _output_get (Variables|Default|SetAs%20BP%20Character _asbp_character))
  (EventDispatchers|BindEventtoGetProduct _output_get (EventDispatchers|CreateEvent :!event Custom|CountingProductsTaken)))

(fn ConstructionScript
  (|CallParentFunction))